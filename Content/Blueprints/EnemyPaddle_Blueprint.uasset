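; Enemy paddle Blueprint that acts as a simple AI opponent in a Pong-style ball game.
; Each Tick it finds the tagged ball actor and moves the paddle up or down toward the ball's height with a swept move, scaled by delta time and EnemyMoveSpeed.
; SpeedUp raises that speed in fixed steps, meant for each ball hit, and ResetSpeed restores it to a set value.
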(event `self.ReceiveTick`
  (params (DeltaSeconds :type "Float (single-precision)"))
  (bind _paddle (`self.Paddle`))
  (bind (_returnvalue_x _returnvalue_y _returnvalue_z) (`KismetMathLibrary.BreakVector` (`SceneComponent.K2_GetComponentLocation` (`self.Paddle`))))
  ;[1 1 1] The "AI" for the enemy paddle. I didn't have the time to figure out just how I would have gotten the enemy AI to work without creating a new blueprint, so here we are. It works though ¯\_(ツ)_/¯
  (bind _outactors (`GameplayStatics.GetAllActorsOfClassWithTag` "/Game/Blueprints/Ball_Blueprint.Ball_Blueprint_C" "Ball"))
  (bind (_returnvalue_x_2 _returnvalue_y_2 _returnvalue_z_2) (`KismetMathLibrary.BreakVector` (`self.K2_GetActorLocation` (`|GetArrayItem` _outactors))))
  (`/Engine/EditorBlueprintResources/StandardMacros.CompareFloat` _returnvalue_z_2 _returnvalue_z
    (:`>`
      (`SceneComponent.K2_SetWorldLocation` _paddle (+ (`KismetMathLibrary.MakeVector` _returnvalue_x _returnvalue_y _returnvalue_z) (`KismetMathLibrary.MakeVector` 0.0 0.0 (* DeltaSeconds (* (`self.EnemyMoveSpeed`) 1.0)))) true false))
    (:`<`
      (`SceneComponent.K2_SetWorldLocation` _paddle (+ (`KismetMathLibrary.MakeVector` _returnvalue_x _returnvalue_y _returnvalue_z) (`KismetMathLibrary.MakeVector` 0.0 0.0 (* DeltaSeconds (* (`self.EnemyMoveSpeed`) -1.0)))) true false))))

(event `SpeedUp`
  ;[1 1 1] The enemy speeds up everytime it hits the ball!
  (set `self.EnemyMoveSpeed` (+ 5.0 (`self.EnemyMoveSpeed`))))

(event `ResetSpeed`
  ;[1 1 1] Reset movement speed
  (set `self.EnemyMoveSpeed` 50.0))

(fn `UserConstructionScript`
  (`parent.UserConstructionScript`))