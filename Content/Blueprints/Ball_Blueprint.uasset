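; Pong-style ball that moves on Tick, bounces, and also owns both scores and creates the score widget on BeginPlay.
; Hitbox overlaps branch on component tags: walls flip Z velocity, while paddles set direction from the YZ offset between paddle and ball.
; Each paddle hit speeds up the ball, and enemy hits also speed up that paddle.
; Side zones award the opposing score, then reset the ball and enemy paddle speed.
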(event `self.ReceiveBeginPlay`
  ;[1 1 1] Setting up initial ball velocity and speed
  (set `self.BallSpeed` 100.0)
  (set `self.BallVelocityVector` (0.0 -1.0 0.0))
  ;[1 1 1] Your UI are now belong to the ball. Sorry!
  (bind _returnvalue (`|CreateWidget` "/Game/Blueprints/ScoreInterface_Blueprint.ScoreInterface_Blueprint_C"))
  (`UserWidget.AddToViewport` _returnvalue 0))

(event `self.ReceiveTick`
  (params (DeltaSeconds :type "Float (single-precision)"))
  (bind _ball (`self.Ball`))
  ;[1 1 1] Ball movement. Event Tick is apparenly the same as Unity's Update()-method
  (`KismetSystemLibrary.FlushDebugStrings`)
  (`SceneComponent.K2_SetWorldLocation` _ball (+ (`SceneComponent.K2_GetComponentLocation` _ball) (* (* (`self.BallVelocityVector`) (`self.BallSpeed`)) DeltaSeconds)) true false))

(event `self.hitbox.OnComponentBeginOverlap`
  (params (OverlappedComponent :type "PrimitiveComponent Object Reference") (OtherActor :type "Actor Object Reference") (OtherComp :type "PrimitiveComponent Object Reference") (OtherBodyIndex :type Integer) (bFromSweep :type Boolean) (SweepResult :type "HitResult Structure (by ref)"))
  (bind (_returnvalue_x _returnvalue_y _returnvalue_z) (`KismetMathLibrary.BreakVector` (`self.K2_GetActorLocation` OtherActor)))
  (bind (_returnvalue_x_2 _returnvalue_y_2 _returnvalue_z_2) (`KismetMathLibrary.BreakVector` (`self.K2_GetActorLocation`)))
  (bind (_ballvelocityvector_x _ballvelocityvector_y _ballvelocityvector_z) (`KismetMathLibrary.BreakVector` (`self.BallVelocityVector`)))
  ;[1 1 1] If we hit a wall, the ball bounces off of it with the same exit angle as the entry angle
  (if (`ActorComponent.ComponentHasTag` OtherComp "Wall")
    (`KismetSystemLibrary.PrintString` "Hit a wall!")
    (set `self.BallVelocityVector` (`KismetMathLibrary.MakeVector` _ballvelocityvector_x _ballvelocityvector_y (* _ballvelocityvector_z -1.0)))
    (else
      ;[1 1 1] If we hit a paddle, we bounce at an approriate angle
      (if (`ActorComponent.ComponentHasTag` OtherComp "Paddle")
        (`KismetSystemLibrary.PrintString` "Hit a paddle!")
        (set `self.BallVelocityVector` (`KismetMathLibrary.Normal` (- (`KismetMathLibrary.MakeVector` 0.0 _returnvalue_y_2 _returnvalue_z_2) (`KismetMathLibrary.MakeVector` 0.0 _returnvalue_y _returnvalue_z))))
        ;[1 1 1] The ball speeds up every time it hits a paddle!
        (set `self.BallSpeed` (+ 10.0 (`self.BallSpeed`)))
        ;[1 1 1] The enemy also speeds up everytime it hits the ball!
        (if (`self.ActorHasTag` OtherActor "EnemyPaddle")
          (bind _asenemy_paddle_blueprint (cast `/Game/Blueprints/EnemyPaddle_Blueprint` OtherActor))
          (`/Game/Blueprints/EnemyPaddle_Blueprint.SpeedUp` _asenemy_paddle_blueprint))
        (else
          ;[1 1 1] The scoring and ball reset system. Didn't have the time to figure out how to bind player scores to the "real players", so they're tied to the ball instead. Now this is what I call spaghetti!
          (if (`ActorComponent.ComponentHasTag` OtherComp "PlayerSide")
            (`KismetSystemLibrary.PrintString` "Enemy scoreded!")
            (bind _result (`/Engine/EditorBlueprintResources/StandardMacros.IncrementInt` (`self.EnemyScore`))
              (:`  `
                (bind _output_get (set `self.EnemyScore` _result))
                (`KismetSystemLibrary.PrintString` (`KismetStringLibrary.Conv_IntToString` _output_get))
                (`SceneComponent.K2_SetWorldLocation` (`self.Ball`) (`self.StartPos`) false true :!label _label)
                (set `self.BallVelocityVector` (0.0 -1.0 0.0))
                (set `self.BallSpeed` 100.0)
                ;[1 1 1] Reset enemy paddle speed
                (bind _outactors (`GameplayStatics.GetAllActorsWithTag` "EnemyPaddle"))
                (bind _asenemy_paddle_blueprint_2 (cast `/Game/Blueprints/EnemyPaddle_Blueprint` (`|GetArrayItem` _outactors)))
                (`/Game/Blueprints/EnemyPaddle_Blueprint.ResetSpeed` _asenemy_paddle_blueprint_2)
                (`KismetSystemLibrary.PrintString` "Resetting enemy paddle movement speed")))
            (elif (`ActorComponent.ComponentHasTag` OtherComp "EnemySide")
              (`KismetSystemLibrary.PrintString` "Player Scoreded!")
              (bind _result_2 (`/Engine/EditorBlueprintResources/StandardMacros.IncrementInt` (`self.PlayerScore`))
                (:`  `
                  (bind _output_get_2 (set `self.PlayerScore` _result_2))
                  (`KismetSystemLibrary.PrintString` (`KismetStringLibrary.Conv_IntToString` _output_get_2))
                  (goto _label))))))))))

(fn `UserConstructionScript`)